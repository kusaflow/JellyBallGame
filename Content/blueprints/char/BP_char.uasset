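; BP_char is a character test Blueprint that drives part of its skeletal mesh with physical animation.
; On BeginPlay it applies the kusaBallP profile below BoneName, simulates physics beneath that bone excluding itself, then sets the kusaBallC constraint profile.
; Pressing W applies a large, mostly upward velocity-change impulse to the mesh.
; An unconnected node holds hand-set physical animation settings as an alternative to the profile.
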(event EventBeginPlay
  (bind _physicalanimation (Variables|Default|GetPhysicalAnimation))
  (bind _mesh (Variables|Character|GetMesh))
  (bind _bonename (Variables|Default|GetboneName))
  (Class|PhysicalAnimationComponent|SetSkeletalMeshComponent _physicalanimation (Variables|Character|GetMesh))
  (Class|PhysicalAnimationComponent|ApplyPhysicalAnimationProfileBelow _physicalanimation _bonename "kusaBallP" true false)
  (Class|SkeletalMeshComponent|SetAllBodiesBelowSimulatePhysics _mesh _bonename true false)
  (Class|SkeletalMeshComponent|SetConstraintProfileforAll _mesh "kusaBallC" false))

(event Collision|EventActorBeginOverlap
  (params (OtherActor :type Actor%20Object%20Reference)))

(event EventTick
  (params (DeltaSeconds :type Float%20%28single-precision%29)))

(event Input|KeyboardEvents|W
  (params (Key :type Key%20Structure :default "None"))
  (:Pressed
    (Physics|AddImpulse (Variables|Character|GetMesh) "500.000000, 0,5000.000000" "None" true)))

(fn ConstructionScript)